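; Gunsmith Blueprint that switches the player's view between weapon customization cameras for the barrel, whole gun, sight and under-gun views.
; Each CameraChangeTo function calls SetViewTargetWithBlend on the first player controller, using its matching camera actor and a short timed blend.
; The event graph and construction script hold no active logic, so switching relies on these functions being called from elsewhere.
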(fn `CameraChangeToBarrel`
  (`PlayerController.SetViewTargetWithBlend` (`GameplayStatics.GetPlayerController` 0) (`self.CameraActorBarrel`) 0.5 "VTBlend_Linear" 0.0 false))

(fn `CameraChangeToGun`
  (`PlayerController.SetViewTargetWithBlend` (`GameplayStatics.GetPlayerController` 0) (`self.CameraActorGun`) 0.5 "VTBlend_Linear" 0.0 false))

(fn `CameraChangeToSight`
  (`PlayerController.SetViewTargetWithBlend` (`GameplayStatics.GetPlayerController` 0) (`self.CameraActorSight`) 0.5 "VTBlend_Linear" 0.0 false))

(fn `CameraChangeToUnder`
  (`PlayerController.SetViewTargetWithBlend` (`GameplayStatics.GetPlayerController` 0) (`self.CameraActorUnder`) 0.5 "VTBlend_Linear" 0.0 false))

(fn `UserConstructionScript`)