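; BP_Weapon is the gunsmith display weapon, rebuilding its look from the player's UI selections stored in GM_Gunsmith.
; On the game mode's UI input event, it swaps the skeletal mesh, creates three dynamic material instances for paint, then sets scope, underbarrel and barrel meshes.
; Weapon-incompatible attachments update the UI buttons and re-run their switch, with scope and underbarrel falling back to None and barrel to the previous selection.
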(event `self.ReceiveBeginPlay`
  (bind _asgm_gunsmith (cast `/Game/Gunsmith/Blueprints/GM_Gunsmith` (`GameplayStatics.GetGameMode`)))
  (bind _output_get (set `self.As GM Gunsmith` _asgm_gunsmith))
  (add `/Game/Gunsmith/Blueprints/GM_Gunsmith.ED_UiInput` _output_get (delegate `CE_UiInput`)))

(event `CE_UiInput`
  (bind _weaponmesh (`self.WeaponMesh`))
  (bind _dynmat2 (`self.DynMat2`))
  (bind _dynmat (`self.DynMat`))
  (bind _dynmat3 (`self.DynMat3`))
  (bind _weaponmesh_2 (`self.WeaponMesh`))
  (bind _weaponmesh_3 (`self.WeaponMesh`))
  (bind _as_gm_gunsmith (`self.As GM Gunsmith`))
  (bind _as_gm_gunsmith_2 (`self.As GM Gunsmith`))
  (bind _as_gm_gunsmith_3 (`self.As GM Gunsmith`))
  (bind _as_gm_gunsmith_4 (`self.As GM Gunsmith`))
  (bind _as_gm_gunsmith_5 (`self.As GM Gunsmith`))
  (bind _weaponmesh_4 (`self.WeaponMesh`))
  (bind _as_gm_gunsmith_6 (`self.As GM Gunsmith`))
  (bind _as_gm_gunsmith_7 (`self.As GM Gunsmith`))
  (bind _weaponmesh_5 (`self.WeaponMesh`))
  (bind _weaponmesh_6 (`self.WeaponMesh`))
  (bind _dynmat_2 (`self.DynMat`))
  (bind _dynmat2_2 (`self.DynMat2`))
  (bind _dynmat3_2 (`self.DynMat3`))
  (bind _dynmat_3 (`self.DynMat`))
  (bind _dynmat2_3 (`self.DynMat2`))
  (bind _dynmat3_3 (`self.DynMat3`))
  (bind _dynmat_4 (`self.DynMat`))
  (bind _dynmat2_4 (`self.DynMat2`))
  (bind _dynmat3_4 (`self.DynMat3`))
  (bind _dynmat_5 (`self.DynMat`))
  (bind _dynmat2_5 (`self.DynMat2`))
  (bind _dynmat3_5 (`self.DynMat3`))
  (`|ExecutionSequence`
    (:`then_0`
      (switch `/Game/Gunsmith/Blueprints/Enumerations/EN_WeaponList` (`/Game/Gunsmith/Blueprints/GM_Gunsmith.WeaponSelected` (`self.As GM Gunsmith`))
        (:`NewEnumerator0`
          ;[1 1 1] Display Service Weapon w/ its materials
          (`SkinnedMeshComponent.SetSkinnedAssetAndUpdate` _weaponmesh_2 "/Game/Gunsmith/Meshes/Benitez_ServiceWeapon.Benitez_ServiceWeapon" true)
          (bind _returnvalue (`PrimitiveComponent.CreateDynamicMaterialInstance` _weaponmesh_2 0 "/Game/Gunsmith/Materials/MI_SW_Grip.MI_SW_Grip" "None"))
          (set `self.DynMat` _returnvalue)
          (bind _returnvalue_2 (`PrimitiveComponent.CreateDynamicMaterialInstance` _weaponmesh_2 1 "/Game/Gunsmith/Materials/MI_SW_Metal.MI_SW_Metal" "None"))
          (set `self.DynMat2` _returnvalue_2)
          (bind _returnvalue_3 (`PrimitiveComponent.CreateDynamicMaterialInstance` _weaponmesh_2 2 "/Game/Gunsmith/Materials/MI_SAR_Mag.MI_SAR_Mag" "None"))
          (set `self.DynMat3` _returnvalue_3))
        (:`NewEnumerator1`
          ;[1 1 1] Display Flintlock w/ its materials
          (`SkinnedMeshComponent.SetSkinnedAssetAndUpdate` _weaponmesh "/Game/Gunsmith/Meshes/FlintLock.FlintLock" true)
          (bind _returnvalue_4 (`PrimitiveComponent.CreateDynamicMaterialInstance` _weaponmesh 0 "/Game/Gunsmith/Materials/MI_Flintlock_M2.MI_Flintlock_M2" "None"))
          (set `self.DynMat` _returnvalue_4)
          (bind _returnvalue_5 (`PrimitiveComponent.CreateDynamicMaterialInstance` _weaponmesh 1 "/Game/Gunsmith/Materials/MI_Flintlock_M1.MI_Flintlock_M1" "None"))
          (set `self.DynMat2` _returnvalue_5)
          (bind _returnvalue_6 (`PrimitiveComponent.CreateDynamicMaterialInstance` _weaponmesh 2 "/Game/Gunsmith/Materials/MI_SAR_Mag.MI_SAR_Mag" "None"))
          (set `self.DynMat3` _returnvalue_6))
        (:`NewEnumerator2`
          ;[1 1 1] Display MAC10 w/ its materials
          (`SkinnedMeshComponent.SetSkinnedAssetAndUpdate` _weaponmesh_3 "/Game/Gunsmith/Meshes/Peloquin_Mac10.Peloquin_Mac10" true)
          (bind _returnvalue_7 (`PrimitiveComponent.CreateDynamicMaterialInstance` _weaponmesh_3 0 "/Game/Gunsmith/Materials/MI_MAC_M2.MI_MAC_M2" "None"))
          (set `self.DynMat` _returnvalue_7)
          (bind _returnvalue_8 (`PrimitiveComponent.CreateDynamicMaterialInstance` _weaponmesh_3 1 "/Game/Gunsmith/Materials/MI_MAC10_M1.MI_MAC10_M1" "None"))
          (set `self.DynMat2` _returnvalue_8)
          (bind _returnvalue_9 (`PrimitiveComponent.CreateDynamicMaterialInstance` _weaponmesh_3 2 "/Game/Gunsmith/Materials/MI_SAR_Mag.MI_SAR_Mag" "None"))
          (set `self.DynMat3` _returnvalue_9))
        (:`NewEnumerator3`
          ;[1 1 1] Display SAR w/ its materials
          (`SkinnedMeshComponent.SetSkinnedAssetAndUpdate` _weaponmesh_6 "/Game/Gunsmith/Meshes/Popowycz_SAR.Popowycz_SAR" true)
          (bind _returnvalue_10 (`PrimitiveComponent.CreateDynamicMaterialInstance` _weaponmesh_6 0 "/Game/Gunsmith/Materials/MI_SAR_Reciever.MI_SAR_Reciever" "None"))
          (set `self.DynMat` _returnvalue_10)
          (bind _returnvalue_11 (`PrimitiveComponent.CreateDynamicMaterialInstance` _weaponmesh_6 1 "/Game/Gunsmith/Materials/MI_SAR_Barrel.MI_SAR_Barrel" "None"))
          (set `self.DynMat2` _returnvalue_11)
          (bind _returnvalue_12 (`PrimitiveComponent.CreateDynamicMaterialInstance` _weaponmesh_6 2 "/Game/Gunsmith/Materials/MI_SAR_Mag.MI_SAR_Mag" "None"))
          (set `self.DynMat3` _returnvalue_12))
        (:`NewEnumerator4`
          ;[1 1 1] Display Maggie w/ its materials
          (`SkinnedMeshComponent.SetSkinnedAssetAndUpdate` _weaponmesh_4 "/Game/Gunsmith/Meshes/Xia_Maggie.Xia_Maggie" true)
          (bind _returnvalue_13 (`PrimitiveComponent.CreateDynamicMaterialInstance` _weaponmesh_4 0 "/Game/Gunsmith/Materials/MI_Maggie_M2.MI_Maggie_M2" "None"))
          (set `self.DynMat` _returnvalue_13)
          (bind _returnvalue_14 (`PrimitiveComponent.CreateDynamicMaterialInstance` _weaponmesh_4 1 "/Game/Gunsmith/Materials/MI_Maggie_M1.MI_Maggie_M1" "None"))
          (set `self.DynMat2` _returnvalue_14)
          (bind _returnvalue_15 (`PrimitiveComponent.CreateDynamicMaterialInstance` _weaponmesh_4 2 "/Game/Gunsmith/Materials/MI_SAR_Mag.MI_SAR_Mag" "None"))
          (set `self.DynMat3` _returnvalue_15))
        (:`NewEnumerator5`
          ;[1 1 1] Display Harpoon w/ its materials
          (`SkinnedMeshComponent.SetSkinnedAssetAndUpdate` _weaponmesh_5 "/Game/Gunsmith/Meshes/HarpoonGun.HarpoonGun" true)
          (bind _returnvalue_16 (`PrimitiveComponent.CreateDynamicMaterialInstance` _weaponmesh_5 0 "/Game/Gunsmith/Materials/MI_Harpoon_M2.MI_Harpoon_M2" "None"))
          (set `self.DynMat` _returnvalue_16)
          (bind _returnvalue_17 (`PrimitiveComponent.CreateDynamicMaterialInstance` _weaponmesh_5 1 "/Game/Gunsmith/Materials/MI_Harpoon_M3.MI_Harpoon_M3" "None"))
          (set `self.DynMat2` _returnvalue_17)
          (bind _returnvalue_18 (`PrimitiveComponent.CreateDynamicMaterialInstance` _weaponmesh_5 2 "/Game/Gunsmith/Materials/MI_Harpoon_M1.MI_Harpoon_M1" "None"))
          (set `self.DynMat3` _returnvalue_18))))
    (:`then_1`
      (switch `/Game/Gunsmith/Blueprints/Enumerations/EN_PaintList` (`/Game/Gunsmith/Blueprints/GM_Gunsmith.PaintSelected` (`self.As GM Gunsmith`))
        (:`NewEnumerator1`
          ;[1 1 1] Remove paintjob
          (`MaterialInstanceDynamic.SetScalarParameterValue` (`self.DynMat`) "Painted?" 1.0)
          (`MaterialInstanceDynamic.SetScalarParameterValue` (`self.DynMat2`) "Painted?" 1.0)
          (`MaterialInstanceDynamic.SetScalarParameterValue` (`self.DynMat3`) "Painted?" 1.0))
        (:`NewEnumerator0`
          ;[1 1 1] Set paint to Cool Blue
          (`MaterialInstanceDynamic.SetScalarParameterValue` _dynmat_2 "Painted?" 0.0)
          (`MaterialInstanceDynamic.SetVectorParameterValue` _dynmat_2 "PaintColor" (struct :`R` 0.003922 :`B` 0.2 :`A` 1.0))
          (`MaterialInstanceDynamic.SetScalarParameterValue` _dynmat2_2 "Painted?" 0.0)
          (`MaterialInstanceDynamic.SetVectorParameterValue` _dynmat2_2 "PaintColor" (struct :`R` 0.003922 :`B` 0.2 :`A` 1.0))
          (`MaterialInstanceDynamic.SetScalarParameterValue` _dynmat3_2 "Painted?" 0.0)
          (`MaterialInstanceDynamic.SetVectorParameterValue` _dynmat3_2 "PaintColor" (struct :`R` 0.003922 :`B` 0.2 :`A` 1.0)))
        (:`NewEnumerator2`
          ;[1 1 1] Set paint to Army Green
          (`MaterialInstanceDynamic.SetScalarParameterValue` _dynmat_3 "Painted?" 0.0)
          (`MaterialInstanceDynamic.SetVectorParameterValue` _dynmat_3 "PaintColor" (struct :`R` 0.133333 :`G` 0.168627 :`B` 0.062745 :`A` 1.0))
          (`MaterialInstanceDynamic.SetScalarParameterValue` _dynmat2_3 "Painted?" 0.0)
          (`MaterialInstanceDynamic.SetVectorParameterValue` _dynmat2_3 "PaintColor" (struct :`R` 0.133333 :`G` 0.168627 :`B` 0.062745 :`A` 1.0))
          (`MaterialInstanceDynamic.SetScalarParameterValue` _dynmat3_3 "Painted?" 0.0)
          (`MaterialInstanceDynamic.SetVectorParameterValue` _dynmat3_3 "PaintColor" (struct :`R` 0.133333 :`G` 0.168627 :`B` 0.062745 :`A` 1.0)))
        (:`NewEnumerator3`
          ;[1 1 1] Set paint to Hot Pink
          (`MaterialInstanceDynamic.SetScalarParameterValue` _dynmat_4 "Painted?" 0.0)
          (`MaterialInstanceDynamic.SetVectorParameterValue` _dynmat_4 "PaintColor" (struct :`R` 1.0 :`G` 0.007843 :`B` 0.886275 :`A` 1.0))
          (`MaterialInstanceDynamic.SetScalarParameterValue` _dynmat2_4 "Painted?" 0.0)
          (`MaterialInstanceDynamic.SetVectorParameterValue` _dynmat2_4 "PaintColor" (struct :`R` 1.0 :`G` 0.007843 :`B` 0.886275 :`A` 1.0))
          (`MaterialInstanceDynamic.SetScalarParameterValue` _dynmat3_4 "Painted?" 0.0)
          (`MaterialInstanceDynamic.SetVectorParameterValue` _dynmat3_4 "PaintColor" (struct :`R` 1.0 :`G` 0.007843 :`B` 0.886275 :`A` 1.0)))
        (:`NewEnumerator4`
          ;[1 1 1] Set paint to Blood Red
          (`MaterialInstanceDynamic.SetScalarParameterValue` _dynmat_5 "Painted?" 0.0)
          (`MaterialInstanceDynamic.SetVectorParameterValue` _dynmat_5 "PaintColor" (struct :`R` 0.301961 :`B` 0.003922 :`A` 1.0))
          (`MaterialInstanceDynamic.SetScalarParameterValue` _dynmat2_5 "Painted?" 0.0)
          (`MaterialInstanceDynamic.SetVectorParameterValue` _dynmat2_5 "PaintColor" (struct :`R` 0.301961 :`B` 0.003922 :`A` 1.0))
          (`MaterialInstanceDynamic.SetScalarParameterValue` _dynmat3_5 "Painted?" 0.0)
          (`MaterialInstanceDynamic.SetVectorParameterValue` _dynmat3_5 "PaintColor" (struct :`R` 0.301961 :`B` 0.003922 :`A` 1.0)))
        (:`NewEnumerator5`
          ;[1 1 1] Set paint to Blackout
          (`MaterialInstanceDynamic.SetScalarParameterValue` _dynmat "Painted?" 0.0)
          (`MaterialInstanceDynamic.SetVectorParameterValue` _dynmat "PaintColor" (struct :`A` 1.0))
          (`MaterialInstanceDynamic.SetScalarParameterValue` _dynmat2 "Painted?" 0.0)
          (`MaterialInstanceDynamic.SetVectorParameterValue` _dynmat2 "PaintColor" (struct :`A` 1.0))
          (`MaterialInstanceDynamic.SetScalarParameterValue` _dynmat3 "Painted?" 0.0)
          (`MaterialInstanceDynamic.SetVectorParameterValue` _dynmat3 "PaintColor" (struct :`A` 1.0)))))
    (:`then_2`
      (switch `/Game/Gunsmith/Blueprints/Enumerations/EN_ScopeList` (`/Game/Gunsmith/Blueprints/GM_Gunsmith.ScopeSelected` (`self.As GM Gunsmith`)) :!label _label
        (:`NewEnumerator2`
          ;[1 1 1] Remove Scope
          (`StaticMeshComponent.SetStaticMesh` (`self.ScopeAttachment`) null))
        (:`NewEnumerator0`
          ;[1 1 1] Set Scope to Holosight (except for MAC10)
          (if (`|EnumEquality` (`/Game/Gunsmith/Blueprints/GM_Gunsmith.WeaponSelected` (`self.As GM Gunsmith`)) "NewEnumerator2")
            (set `/Game/Gunsmith/Blueprints/GM_Gunsmith.ScopeSelected` "NewEnumerator2" _as_gm_gunsmith_3)
            (set `self.Temp` (`/Game/Gunsmith/Blueprints/GM_Gunsmith.LastButtonScope` _as_gm_gunsmith_3))
            (bind _output_get (set `/Game/Gunsmith/Blueprints/GM_Gunsmith.LastButtonScope` (`/Game/Gunsmith/Blueprints/GM_Gunsmith.CurrentButtonScope` _as_gm_gunsmith_3) _as_gm_gunsmith_3))
            (`Widget.SetIsEnabled` _output_get true)
            (bind _output_get_2 (set `/Game/Gunsmith/Blueprints/GM_Gunsmith.CurrentButtonScope` (`/Game/Gunsmith/Blueprints/GM_Gunsmith.NoneScope` _as_gm_gunsmith_3) _as_gm_gunsmith_3))
            (`Widget.SetIsEnabled` _output_get_2 false)
            (goto _label)
            (else
              (`StaticMeshComponent.SetStaticMesh` (`self.ScopeAttachment`) "/Game/Gunsmith/Meshes/Benitez_Holosight.Benitez_Holosight"))))
        (:`NewEnumerator1`
          ;[1 1 1] Set Scope to Laser (except for MAC10)
          (if (`|EnumEquality` (`/Game/Gunsmith/Blueprints/GM_Gunsmith.WeaponSelected` (`self.As GM Gunsmith`)) "NewEnumerator2")
            (set `/Game/Gunsmith/Blueprints/GM_Gunsmith.ScopeSelected` "NewEnumerator2" _as_gm_gunsmith_2)
            (set `self.Temp` (`/Game/Gunsmith/Blueprints/GM_Gunsmith.LastButtonScope` _as_gm_gunsmith_2))
            (bind _output_get_3 (set `/Game/Gunsmith/Blueprints/GM_Gunsmith.LastButtonScope` (`/Game/Gunsmith/Blueprints/GM_Gunsmith.CurrentButtonScope` _as_gm_gunsmith_2) _as_gm_gunsmith_2))
            (`Widget.SetIsEnabled` _output_get_3 true)
            (bind _output_get_4 (set `/Game/Gunsmith/Blueprints/GM_Gunsmith.CurrentButtonScope` (`/Game/Gunsmith/Blueprints/GM_Gunsmith.NoneScope` _as_gm_gunsmith_2) _as_gm_gunsmith_2))
            (`Widget.SetIsEnabled` _output_get_4 false)
            (goto _label)
            (else
              (`StaticMeshComponent.SetStaticMesh` (`self.ScopeAttachment`) "/Game/Gunsmith/Meshes/Laser.Laser"))))
        (:`NewEnumerator3`
          ;[1 1 1] Set Scope to Reflex Sight
          (`StaticMeshComponent.SetStaticMesh` (`self.ScopeAttachment`) "/Game/Gunsmith/Meshes/Peloquin_ReflexSight.Peloquin_ReflexSight"))
        (:`NewEnumerator4`
          ;[1 1 1] Set Scope to Handmade Scope
          (if (`|EnumEquality` (`/Game/Gunsmith/Blueprints/GM_Gunsmith.WeaponSelected` (`self.As GM Gunsmith`)) "NewEnumerator2")
            (set `/Game/Gunsmith/Blueprints/GM_Gunsmith.ScopeSelected` "NewEnumerator2" _as_gm_gunsmith_5)
            (set `self.Temp` (`/Game/Gunsmith/Blueprints/GM_Gunsmith.LastButtonScope` _as_gm_gunsmith_5))
            (bind _output_get_5 (set `/Game/Gunsmith/Blueprints/GM_Gunsmith.LastButtonScope` (`/Game/Gunsmith/Blueprints/GM_Gunsmith.CurrentButtonScope` _as_gm_gunsmith_5) _as_gm_gunsmith_5))
            (`Widget.SetIsEnabled` _output_get_5 true)
            (bind _output_get_6 (set `/Game/Gunsmith/Blueprints/GM_Gunsmith.CurrentButtonScope` (`/Game/Gunsmith/Blueprints/GM_Gunsmith.NoneScope` _as_gm_gunsmith_5) _as_gm_gunsmith_5))
            (`Widget.SetIsEnabled` _output_get_6 false)
            (goto _label)
            (else
              (`StaticMeshComponent.SetStaticMesh` (`self.ScopeAttachment`) "/Game/Gunsmith/Meshes/Popowycz_HandmadeScope.Popowycz_HandmadeScope"))))
        (:`NewEnumerator5`
          ;[1 1 1] Set Scope to Maggie Scope
          (`StaticMeshComponent.SetStaticMesh` (`self.ScopeAttachment`) "/Game/Gunsmith/Meshes/Xia_Scope.Xia_Scope"))
        (:`NewEnumerator6`
          ;[1 1 1] Set Scope to Spy Glass Scope
          (if (`|EnumEquality` (`/Game/Gunsmith/Blueprints/GM_Gunsmith.WeaponSelected` (`self.As GM Gunsmith`)) "NewEnumerator2")
            (set `/Game/Gunsmith/Blueprints/GM_Gunsmith.ScopeSelected` "NewEnumerator2" _as_gm_gunsmith :!label _label_2)
            (set `self.Temp` (`/Game/Gunsmith/Blueprints/GM_Gunsmith.LastButtonScope` _as_gm_gunsmith))
            (bind _output_get_7 (set `/Game/Gunsmith/Blueprints/GM_Gunsmith.LastButtonScope` (`/Game/Gunsmith/Blueprints/GM_Gunsmith.CurrentButtonScope` _as_gm_gunsmith) _as_gm_gunsmith))
            (`Widget.SetIsEnabled` _output_get_7 true)
            (bind _output_get_8 (set `/Game/Gunsmith/Blueprints/GM_Gunsmith.CurrentButtonScope` (`/Game/Gunsmith/Blueprints/GM_Gunsmith.NoneScope` _as_gm_gunsmith) _as_gm_gunsmith))
            (`Widget.SetIsEnabled` _output_get_8 false)
            (goto _label)
            (elif (`|EnumEquality` (`/Game/Gunsmith/Blueprints/GM_Gunsmith.WeaponSelected` (`self.As GM Gunsmith`)) "NewEnumerator0")
              (goto _label_2)
              (else
                (`StaticMeshComponent.SetStaticMesh` (`self.ScopeAttachment`) "/Game/Gunsmith/Meshes/SpyGlassScope.SpyGlassScope")))))))
    (:`then_3`
      (switch `/Game/Gunsmith/Blueprints/Enumerations/EN_UnderbarrelList` (`/Game/Gunsmith/Blueprints/GM_Gunsmith.UnderbarrelSelected` (`self.As GM Gunsmith`)) :!label _label_3
        (:`NewEnumerator0`
          ;[1 1 1] Remove Underbarrel
          (`StaticMeshComponent.SetStaticMesh` (`self.UnderbarrelAttachment`) null))
        (:`NewEnumerator1`
          ;[1 1 1] Set Underbarrel to Foregrip (only for SAR)
          (if (`|EnumEquality` (`/Game/Gunsmith/Blueprints/GM_Gunsmith.WeaponSelected` _as_gm_gunsmith_6) "NewEnumerator3")
            (`StaticMeshComponent.SetStaticMesh` (`self.UnderbarrelAttachment`) "/Game/Gunsmith/Meshes/Popowycz_HandmadeForegrip.Popowycz_HandmadeForegrip")
            (else
              (set `/Game/Gunsmith/Blueprints/GM_Gunsmith.UnderbarrelSelected` "NewEnumerator0" _as_gm_gunsmith_6)
              (set `self.Temp` (`/Game/Gunsmith/Blueprints/GM_Gunsmith.LastButtonUnderbarrel` _as_gm_gunsmith_6))
              (bind _output_get_9 (set `/Game/Gunsmith/Blueprints/GM_Gunsmith.LastButtonUnderbarrel` (`/Game/Gunsmith/Blueprints/GM_Gunsmith.CurrentButtonUnderbarrel` _as_gm_gunsmith_6) _as_gm_gunsmith_6))
              (`Widget.SetIsEnabled` _output_get_9 true)
              (bind _output_get_10 (set `/Game/Gunsmith/Blueprints/GM_Gunsmith.CurrentButtonUnderbarrel` (`/Game/Gunsmith/Blueprints/GM_Gunsmith.NoneUnder` _as_gm_gunsmith_6) _as_gm_gunsmith_6))
              (`Widget.SetIsEnabled` _output_get_10 false)
              (goto _label_3))))
        (:`NewEnumerator2`
          ;[1 1 1] Set Underbarrel to Laser Sight (only for SAR)
          (if (`|EnumEquality` (`/Game/Gunsmith/Blueprints/GM_Gunsmith.WeaponSelected` _as_gm_gunsmith_4) "NewEnumerator3")
            (`StaticMeshComponent.SetStaticMesh` (`self.UnderbarrelAttachment`) "/Game/Gunsmith/Meshes/Laser.Laser")
            (else
              (set `/Game/Gunsmith/Blueprints/GM_Gunsmith.UnderbarrelSelected` "NewEnumerator0" _as_gm_gunsmith_4)
              (set `self.Temp` (`/Game/Gunsmith/Blueprints/GM_Gunsmith.LastButtonUnderbarrel` _as_gm_gunsmith_4))
              (bind _output_get_11 (set `/Game/Gunsmith/Blueprints/GM_Gunsmith.LastButtonUnderbarrel` (`/Game/Gunsmith/Blueprints/GM_Gunsmith.CurrentButtonUnderbarrel` _as_gm_gunsmith_4) _as_gm_gunsmith_4))
              (`Widget.SetIsEnabled` _output_get_11 true)
              (bind _output_get_12 (set `/Game/Gunsmith/Blueprints/GM_Gunsmith.CurrentButtonUnderbarrel` (`/Game/Gunsmith/Blueprints/GM_Gunsmith.NoneUnder` _as_gm_gunsmith_4) _as_gm_gunsmith_4))
              (`Widget.SetIsEnabled` _output_get_12 false)
              (goto _label_3))))))
    (:`then_4`
      (switch `/Game/Gunsmith/Blueprints/Enumerations/EN_BarrelList` (`/Game/Gunsmith/Blueprints/GM_Gunsmith.BarrelSelected` (`self.As GM Gunsmith`)) :!label _label_4
        (:`NewEnumerator0`
          ;[1 1 1] Remove Barrel
          (`StaticMeshComponent.SetStaticMesh` (`self.BarrelAttachment`) null))
        (:`NewEnumerator1`
          ;[1 1 1] Set Barrel to Oily Silence (Except for Service Weapon, Flintlock, and Harpoon)
          (if (`|EnumEquality` (`/Game/Gunsmith/Blueprints/GM_Gunsmith.WeaponSelected` _as_gm_gunsmith_7) "NewEnumerator0")
            (set `/Game/Gunsmith/Blueprints/GM_Gunsmith.BarrelSelected` (`/Game/Gunsmith/Blueprints/GM_Gunsmith.LastBarrel` _as_gm_gunsmith_7) _as_gm_gunsmith_7 :!label _label_5)
            (set `self.Temp` (`/Game/Gunsmith/Blueprints/GM_Gunsmith.LastButtonBarrel` _as_gm_gunsmith_7))
            (bind _output_get_13 (set `/Game/Gunsmith/Blueprints/GM_Gunsmith.LastButtonBarrel` (`/Game/Gunsmith/Blueprints/GM_Gunsmith.CurrentButtonBarrel` _as_gm_gunsmith_7) _as_gm_gunsmith_7))
            (`Widget.SetIsEnabled` _output_get_13 true)
            (bind _output_get_14 (set `/Game/Gunsmith/Blueprints/GM_Gunsmith.CurrentButtonBarrel` (`self.Temp`) _as_gm_gunsmith_7))
            (`Widget.SetIsEnabled` _output_get_14 false)
            (goto _label_4)
            (elif (`|EnumEquality` (`/Game/Gunsmith/Blueprints/GM_Gunsmith.WeaponSelected` _as_gm_gunsmith_7) "NewEnumerator1")
              (goto _label_5)
              (elif (`|EnumEquality` (`/Game/Gunsmith/Blueprints/GM_Gunsmith.WeaponSelected` _as_gm_gunsmith_7) "NewEnumerator5")
                (goto _label_5)
                (else
                  (`StaticMeshComponent.SetStaticMesh` (`self.BarrelAttachment`) "/Game/Gunsmith/Meshes/Popowycz_OilcanSuppressor.Popowycz_OilcanSuppressor"))))))))))

(fn `UserConstructionScript`)